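; MyCollectable3_3 is a pickup actor that destroys its StaticMesh1 component when any actor begins overlapping it.
; It increments the Collectable3 counter on the first MyCollectable3_1 actor found in the level, which serves as the shared tally.
; If the overlapping actor is a MyCharacter, it plays the pickup sound at its location, half-pitched while that character's SlowMotion is active.
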(event OnComponentBeginOverlap(StaticMesh1)
  (params (OtherActor :type Actor%20Object%20Reference) (OtherComp :type Primitive%20Component%20Object%20Reference) (OtherBodyIndex :type Integer) (bFromSweep :type Boolean) (SweepResult :type Hit%20Result%20Structure%20%28by%20ref%29))
  (bind _returnvalue (Transformation|GetActorLocation))
  (Components|DestroyComponent (Variables|Default|GetStaticMesh1))
  (bind _outactors (Actor|GetAllActorsOfClass "/Game/Blueprints/MyCollectable3_1.MyCollectable3_1_C"))
  (bind _asmycollectable3_1_c (Utilities|Casting|CastToMyCollectable3_1 (Utilities|Array|Get(acopy) _outactors)))
  (Variables|/Game/Blueprints/MyCollectable3_1.MyCollectable3_1_C|SetCollectable%203 _asmycollectable3_1_c (+ (Variables|/Game/Blueprints/MyCollectable3_1.MyCollectable3_1_C|GetCollectable%203 _asmycollectable3_1_c) 1))
  (bind _asmycharacter_c (Utilities|Casting|CastToMyCharacter OtherActor))
  (if (Variables|/Game/Blueprints/MyCharacter.MyCharacter_C|GetSlow%20Motion _asmycharacter_c)
    (Audio|PlaySoundatLocation "/Game/Audio/Pickup.Pickup" _returnvalue 1.0 0.5)
    (else
      (Audio|PlaySoundatLocation "/Game/Audio/Pickup.Pickup" _returnvalue 1.0 1.0))))

(fn ConstructionScript)