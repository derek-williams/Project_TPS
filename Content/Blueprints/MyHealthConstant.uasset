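; A healing zone actor that continuously restores the player's Health while MyCharacter stays inside its Box1 trigger.
; Overlap opens a Gate that re-feeds itself through a short Delay, adding one Health per pass until end overlap closes it.
; A DoOnce with delayed reset throttles the heal sound, lowering its pitch and shortening the reset during SlowMotion.
; Tick rotates the whole actor along the camera-to-TextRender direction for billboarding.
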(event OnComponentBeginOverlap(Box1)
  (params (OtherActor :type Actor%20Object%20Reference) (OtherComp :type Primitive%20Component%20Object%20Reference) (OtherBodyIndex :type Integer) (bFromSweep :type Boolean) (SweepResult :type Hit%20Result%20Structure%20%28by%20ref%29))
  (bind _returnvalue (Transformation|GetActorLocation))
  (bind _asmycharacter_c (Utilities|Casting|CastToMyCharacter OtherActor))
  (Utilities|FlowControl|Sequence
    (:then_0
      (goto _label Open))
    (:then_1
      (Utilities|FlowControl|Gate false :!label _label
        (:Exit
          (Variables|/Game/Blueprints/MyCharacter.MyCharacter_C|SetHealth _asmycharacter_c (+ (Variables|/Game/Blueprints/MyCharacter.MyCharacter_C|GetHealth _asmycharacter_c) 1))
          (Utilities|FlowControl|Sequence
            (:then_0
              (Utilities|FlowControl|Delay 0.05)
              (goto _label))
            (:then_1
              (Utilities|FlowControl|DoOnce false :!label _label_2
                (:Completed
                  (if (Variables|/Game/Blueprints/MyCharacter.MyCharacter_C|GetSlow%20Motion _asmycharacter_c)
                    (Audio|PlaySoundatLocation "/Game/Audio/Health.Health" _returnvalue 1.0 0.5)
                    (Utilities|FlowControl|Delay 0.5)
                    (goto _label_2 Reset)
                    (else
                      (Audio|PlaySoundatLocation "/Game/Audio/Health.Health" _returnvalue)
                      (Utilities|FlowControl|Delay 1.0)
                      (goto _label_2 Reset))))))))))))

(event OnComponentEndOverlap(Box1)
  (params (OtherActor :type Actor%20Object%20Reference) (OtherComp :type Primitive%20Component%20Object%20Reference) (OtherBodyIndex :type Integer))
  (bind _returnvalue (Transformation|GetActorLocation))
  (Utilities|FlowControl|Gate false) ; enters at Close
)

(event EventTick
  (params (DeltaSeconds :type Float%20%28single-precision%29))
  ;[1 1 1] Look/Face At Player
  (Transformation|SetActorRotation (Math|Rotator|FindLookatRotation (Transformation|GetActorLocation (Game|GetPlayerCameraManager 0)) (Transformation|GetWorldLocation (Variables|Default|GetTextRender1)))))

(fn ConstructionScript)